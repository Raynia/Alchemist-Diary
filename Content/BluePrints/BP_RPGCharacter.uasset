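; BP_RPGCharacter is an RPG character Blueprint that shows a temporary HUD and tracks health points.
; On BeginPlay it creates the WB_TempCharacterHUD widget, stores it and adds it to the viewport.
; Debug keys P and O raise and lower health by a test amount, with only the increase clamped to the maximum.
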(event `self.ReceiveBeginPlay`
  (bind _returnvalue (`|CreateWidget` "/Game/BluePrints/Widget/WB_TempCharacterHUD.WB_TempCharacterHUD_C"))
  (bind _output_get (set `self.HUD` _returnvalue))
  (`UserWidget.AddToViewport` _output_get 0))

(event `Key|P`
  (params (Key :type "Key Structure"))
  (bind _returnvalue (`KismetMathLibrary.Conv_IntToDouble` (`self.MaxHealthPoint`)))
  (bind _returnvalue_2 (+ (`self.HealthPoint`) (`self.TestHealthReduction`)))
  (:`Pressed`
    (if (<= _returnvalue _returnvalue_2)
      (set `self.HealthPoint` _returnvalue)
      (else
        (set `self.HealthPoint` _returnvalue_2)))))

(event `Key|O`
  (params (Key :type "Key Structure"))
  (:`Pressed`
    (set `self.HealthPoint` (- (`self.HealthPoint`) (`self.TestHealthReduction`)))))

(fn `UserConstructionScript`)